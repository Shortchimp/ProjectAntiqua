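; Save bench actor that lets the player save or rest through a menu.
; Its trigger zone adds a bench input context, sets the player's BenchRef and shows an interact prompt, reversing these on exit.
; UseBench opens the menu in UI-only input and disables trigger collision until Leave or Save closes it.
; Save flags the checkpoint in the save slot and saves through game mode and inventory; Rest calls the game mode's BenchReset.
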(event `self.ReceiveBeginPlay`
  (bind _returnvalue (`|CreateWidget` "/Game/FlexibleCombatSystem/Widgets/WB_InteractButton.WB_InteractButton_C"))
  (set `self.InteractRef` _returnvalue))

(event `self.Trigger Zone.OnComponentBeginOverlap`
  (params (OverlappedComponent :type "PrimitiveComponent Object Reference") (OtherActor :type "Actor Object Reference") (OtherComp :type "PrimitiveComponent Object Reference") (OtherBodyIndex :type Integer) (bFromSweep :type Boolean) (SweepResult :type "HitResult Structure (by ref)"))
  (bind _ascharacter (cast `Character` OtherActor))
  (bind _asplayer_controller (cast `PlayerController` (`Pawn.GetController` _ascharacter)))
  (bind _returnvalue (pcsubsystem `EnhancedInputLocalPlayerSubsystem` _asplayer_controller))
  (`/Engine/EditorBlueprintResources/StandardMacros.IsValid` _returnvalue
    (:`Is Valid`
      (`EnhancedInputSubsystemInterface.AddMappingContext` _returnvalue "/Game/BenchMechanic/IMC_Bench.IMC_Bench" 0 (struct))
      (bind _asbp_player_character (cast `/Game/FlexibleCombatSystem/Blueprints/BP_PlayerCharacter` _ascharacter))
      (set `/Game/FlexibleCombatSystem/Blueprints/BP_PlayerCharacter.BenchRef` self _asbp_player_character)
      (`UserWidget.AddToViewport` (`self.InteractRef`) 0))))

(event `self.Trigger Zone.OnComponentEndOverlap`
  (params (OverlappedComponent :type "PrimitiveComponent Object Reference") (OtherActor :type "Actor Object Reference") (OtherComp :type "PrimitiveComponent Object Reference") (OtherBodyIndex :type Integer))
  (bind _ascharacter (cast `Character` OtherActor))
  (bind _asplayer_controller (cast `PlayerController` (`Pawn.GetController` _ascharacter)))
  (bind _returnvalue (pcsubsystem `EnhancedInputLocalPlayerSubsystem` _asplayer_controller))
  (`/Engine/EditorBlueprintResources/StandardMacros.IsValid` _returnvalue
    (:`Is Valid`
      (`EnhancedInputSubsystemInterface.RemoveMappingContext` _returnvalue "/Game/BenchMechanic/IMC_Bench.IMC_Bench" (struct))
      (bind _asbp_player_character (cast `/Game/FlexibleCombatSystem/Blueprints/BP_PlayerCharacter` _ascharacter))
      (set `/Game/FlexibleCombatSystem/Blueprints/BP_PlayerCharacter.BenchRef` null _asbp_player_character)
      (`Widget.RemoveFromParent` (`self.InteractRef`)))))

(event `UseBench`
  (bind _returnvalue (`GameplayStatics.GetPlayerController` 0))
  (bind _benchmenuref (`self.BenchMenuRef`))
  (`Widget.RemoveFromParent` (`self.InteractRef`))
  (bind _returnvalue_2 (`|CreateWidget` "/Game/FlexibleCombatSystem/Widgets/WB_BenchMenu.WB_BenchMenu_C"))
  (bind _output_get (set `self.BenchMenuRef` _returnvalue_2))
  (`UserWidget.AddToViewport` _output_get 0)
  (`WidgetBlueprintLibrary.SetInputMode_UIOnlyEx` _returnvalue (`/Game/FlexibleCombatSystem/Widgets/WB_BenchMenu.LeaveButton` (`self.BenchMenuRef`)))
  (set `PlayerController.bShowMouseCursor` true _returnvalue)
  (`|ExecutionSequence`
    (:`then_0`
      (add `/Game/FlexibleCombatSystem/Widgets/WB_BenchMenu.OnLeaveButtonPressed` _benchmenuref (`|CreateDelegate` :!event `LeaveButtonPressed`)))
    (:`then_1`
      (add `/Game/FlexibleCombatSystem/Widgets/WB_BenchMenu.OnSaveButtonPressed` _benchmenuref (`|CreateDelegate` :!event `SaveButtonPressed`)))
    (:`then_2`
      (add `/Game/FlexibleCombatSystem/Widgets/WB_BenchMenu.OnRestButtonPressed` _benchmenuref (`|CreateDelegate` :!event `RestButtonPressed`))))
  (`PrimitiveComponent.SetCollisionEnabled` (`self.Trigger Zone`) "NoCollision"))

(event `LeaveButtonPressed`
  (bind _returnvalue (`GameplayStatics.GetPlayerController` 0))
  (`Widget.RemoveFromParent` (`self.BenchMenuRef`))
  (set `self.BenchMenuRef` null)
  (`WidgetBlueprintLibrary.SetInputMode_GameOnly` _returnvalue)
  (set `PlayerController.bShowMouseCursor` false _returnvalue)
  (`PrimitiveComponent.SetCollisionEnabled` (`self.Trigger Zone`) "QueryOnly"))

(event `SaveButtonPressed`
  (`GameplayStatics.PlaySound2D` "/Game/Sound/gate-point-sound-effect.gate-point-sound-effect" 1.0 1.0 0.0 null null)
  (bind _returnvalue (`GameplayStatics.LoadGameFromSlot` "save1"))
  (bind _asbp_save_game (cast `/Game/FlexibleCombatSystem/Blueprints/BP_SaveGame` _returnvalue))
  (set `/Game/FlexibleCombatSystem/Blueprints/BP_SaveGame.UseCheckpoint?` true _asbp_save_game)
  (`GameplayStatics.SaveGameToSlot` null "save1")
  (bind _asbp_game_modee (cast `/Game/FlexibleCombatSystem/Blueprints/BP_GameModee` (`GameplayStatics.GetGameMode`)))
  (`/Game/FlexibleCombatSystem/Blueprints/BP_GameModee.SaveGame` _asbp_game_modee)
  (bind _asbp_player_character (cast `/Game/FlexibleCombatSystem/Blueprints/BP_PlayerCharacter` (`GameplayStatics.GetPlayerCharacter` 0)))
  (`/Game/Inventory/Blueprints/BP_Inventory.Save Inventory` (`/Game/FlexibleCombatSystem/Blueprints/BP_PlayerCharacter.BP_Inventory` _asbp_player_character))
  (`Widget.RemoveFromParent` (`self.BenchMenuRef`))
  (`WidgetBlueprintLibrary.SetInputMode_GameOnly` (`GameplayStatics.GetPlayerController` 0))
  (set `PlayerController.bShowMouseCursor` false (`GameplayStatics.GetPlayerController` 0))
  (`PrimitiveComponent.SetCollisionEnabled` (`self.Trigger Zone`) "QueryOnly"))

(event `RestButtonPressed`
  (`GameplayStatics.PlaySound2D` "/Game/Sound/Button_Press_Sound_Effect.Button_Press_Sound_Effect" 1.0 1.0 0.7 null null)
  (bind _asbp_game_modee (cast `/Game/FlexibleCombatSystem/Blueprints/BP_GameModee` (`GameplayStatics.GetGameMode`)))
  (`/Game/FlexibleCombatSystem/Blueprints/BP_GameModee.BenchReset` _asbp_game_modee))

(fn `UserConstructionScript`)