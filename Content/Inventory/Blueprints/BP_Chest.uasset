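; BP_Chest is an interactable loot chest that holds an array of items and presents them through a WB_Lootbar widget.
; The player entering or leaving its sphere toggles an outline overlay on both chest meshes and the visibility of a widget component.
; Interacting shows the loot bar created at BeginPlay and plays a timeline that pitches the Cube, which Closechest reverses.
; Removeitem overwrites the given slot with a zero-quantity item.
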(event `self.ReceiveBeginPlay`
  (bind _returnvalue (`|CreateWidget` "/Game/Inventory/WidgetBlueprints/WB_Lootbar.WB_Lootbar_C" null self))
  (set `self.lootbarwidget` _returnvalue))

(event `self.Sphere.OnComponentBeginOverlap`
  (params (OverlappedComponent :type "PrimitiveComponent Object Reference") (OtherActor :type "Actor Object Reference") (OtherComp :type "PrimitiveComponent Object Reference") (OtherBodyIndex :type Integer) (bFromSweep :type Boolean) (SweepResult :type "HitResult Structure (by ref)"))
  ;[1 1 1] Highligh object when player enter radius
  (if (== OtherActor (`GameplayStatics.GetPlayerCharacter` 0))
    (`MeshComponent.SetOverlayMaterial` (`self.chestbottom`) "/Game/Inventory/Materials/M_Outline_test.M_Outline_test")
    (`MeshComponent.SetOverlayMaterial` (`self.chesttop`) "/Game/Inventory/Materials/M_Outline_test.M_Outline_test")
    (`SceneComponent.SetVisibility` (`self.Widget`) true false)))

(event `self.Sphere.OnComponentEndOverlap`
  (params (OverlappedComponent :type "PrimitiveComponent Object Reference") (OtherActor :type "Actor Object Reference") (OtherComp :type "PrimitiveComponent Object Reference") (OtherBodyIndex :type Integer))
  ;[1 1 1] Highligh object when player enter radius
  (if (== OtherActor (`GameplayStatics.GetPlayerCharacter` 0))
    (`MeshComponent.SetOverlayMaterial` (`self.chestbottom`) null)
    (`MeshComponent.SetOverlayMaterial` (`self.chesttop`) null)
    (`SceneComponent.SetVisibility` (`self.Widget`) false false)))

(event `Close chest`
  (bind _cube (`self.Cube`))
  (bind (_relativerotation_roll _relativerotation_pitch _relativerotation_yaw) (`KismetMathLibrary.BreakRotator` (`SceneComponent.RelativeRotation` _cube)))
  ;[1 1 1] Open chest
  (bind (_direction _chestfloattrack) (`Timeline|chesttimeline` :!via `Reverse` :!label _label)
    (:`Update`
      (`SceneComponent.K2_SetRelativeRotation` _cube (`KismetMathLibrary.MakeRotator` _relativerotation_roll (`KismetMathLibrary.Lerp` 0.0 60.0 _chestfloattrack) _relativerotation_yaw) false false))))

(event `/Game/Inventory/Blueprints/BPI_Interact_Chest.Interact with Chest`
  ;[1 1 1] Open chest
  (if (not (`Widget.IsVisible` (`self.lootbarwidget`)))
    (`UserWidget.AddToViewport` (`self.lootbarwidget`) 0)
    (goto _label)))

(event `Remove item`
  (params (index :type Integer))
  ;[1 1 1] Remove item from chest
  (`KismetArrayLibrary.Array_Set` (`self.Itemsinchest`) index (make `/Game/Inventory/Structures/S_Itemmaster` (struct))))

(fn `UserConstructionScript`)