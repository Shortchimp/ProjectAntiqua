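; BP_Item is a world pickup item that the player can add to their inventory.
; Its construction script sets the mesh from an Itemdata data table row and enables physics simulation.
; A sphere overlap toggles an outline overlay material and a prompt widget for the player character.
; Interact passes Itemdata to the inventory, then refreshes its UI and destroys the actor on success, or shows a cached inventory-full widget on failure.
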(event `self.Sphere.OnComponentBeginOverlap`
  (params (OverlappedComponent :type "PrimitiveComponent Object Reference") (OtherActor :type "Actor Object Reference") (OtherComp :type "PrimitiveComponent Object Reference") (OtherBodyIndex :type Integer) (bFromSweep :type Boolean) (SweepResult :type "HitResult Structure (by ref)"))
  ;[1 1 1] Highlight Item When Player enters radius
  (if (== OtherActor (`GameplayStatics.GetPlayerCharacter` 0))
    (`MeshComponent.SetOverlayMaterial` (`self.item`) "/Game/Inventory/Materials/M_Outline_test.M_Outline_test")
    (`SceneComponent.SetVisibility` (`self.Widget`) true false)))

(event `self.Sphere.OnComponentEndOverlap`
  (params (OverlappedComponent :type "PrimitiveComponent Object Reference") (OtherActor :type "Actor Object Reference") (OtherComp :type "PrimitiveComponent Object Reference") (OtherBodyIndex :type Integer))
  ;[1 1 1] Highlight Item When Player enters radius
  (if (== OtherActor (`GameplayStatics.GetPlayerCharacter` 0))
    (`MeshComponent.SetOverlayMaterial` (`self.item`) null)
    (`SceneComponent.SetVisibility` (`self.Widget`) false false)))

(event `/Game/Inventory/Blueprints/BP_Interact.Interact`
  (params (BP_Inventory :type "/Game/Inventory/Blueprints/BP_Inventory Object Reference"))
  ;[1 1 1] Pick up item and add to players inventory
  (bind _addeditemtoinventory (`/Game/Inventory/Blueprints/BP_Inventory.Add Item To Inventory` BP_Inventory (`self.Itemdata`)))
  (if _addeditemtoinventory
    (`/Game/Inventory/WidgetBlueprints/WB_Iteminventory.Load Inventory` (`/Game/Inventory/WidgetBlueprints/WB_Inventory.WB_Iteminvetory` (`/Game/Inventory/Blueprints/BP_Inventory.InventoryWidget` BP_Inventory)) BP_Inventory)
    (`self.K2_DestroyActor`)
    (else
      (bind _inventoryfull (`self.Inventoryfull`)
        (:`then`
          (`UserWidget.AddToViewport` _inventoryfull 0)
          (`/Game/Inventory/WidgetBlueprints/WB_InventoryFull.Play animation Event` _inventoryfull))
        (:`else`
          (bind _returnvalue (`|CreateWidget` "/Game/Inventory/WidgetBlueprints/WB_InventoryFull.WB_InventoryFull_C"))
          (bind _output_get (set `self.Inventoryfull` _returnvalue))
          (`UserWidget.AddToViewport` _output_get 0))))))

(fn `UserConstructionScript`
  (bind (_datatable _rowname) (break `DataTableRowHandle` (`.Datatable_2_A422A97947628B14DA2297AF1B0C5536` (break `/Game/Inventory/Structures/S_Itemmaster` (`self.Itemdata`)))))
  (bind _returnvalue (`|GetDataTableRow` _datatable _rowname)
    (:`then`
      (`StaticMeshComponent.SetStaticMesh` (`self.item`) (`.Mesh_16_4C585D5E4F49E75F6A417C9D4F834F81` (break `/Game/Inventory/Structures/S_Item` _returnvalue)))
      (`PrimitiveComponent.SetSimulatePhysics` (`self.item`) true)
      (`PrimitiveComponent.SetSimulatePhysics` (`self.item`) true))))