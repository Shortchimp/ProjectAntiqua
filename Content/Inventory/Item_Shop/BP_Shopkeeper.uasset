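; BP_Shopkeeper is an interactable shopkeeper that opens and closes the shop UI.
; Interacting creates a WB_Shop widget, hands it a reference to the shopkeeper, adds it to the viewport and switches the player to UI-only input with the mouse cursor shown.
; CloseShop removes the widget, restores game-only input and hides the cursor.
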(event `/Game/Inventory/Blueprints/BPI_Interact_Shopkeeper.Interact with Shopkeeper`
  (`self.Show Shop`))

(event `Show Shop`
  (bind _returnvalue (`GameplayStatics.GetPlayerController` 0))
  (bind _returnvalue_2 (`|CreateWidget` "/Game/Inventory/Item_Shop/WB_Shop.WB_Shop_C"))
  (set `/Game/Inventory/Item_Shop/WB_Shop.ShopKeeper` self _returnvalue_2)
  (bind _output_get (set `self.Shop Widget` _returnvalue_2))
  (`UserWidget.AddToViewport` _output_get 0)
  (`WidgetBlueprintLibrary.SetInputMode_UIOnlyEx` _returnvalue _output_get)
  (set `PlayerController.bShowMouseCursor` true _returnvalue))

(fn `Close Shop`
  (bind _returnvalue (`GameplayStatics.GetPlayerController` 0))
  (`Widget.RemoveFromParent` (`self.Shop Widget`))
  (`WidgetBlueprintLibrary.SetInputMode_GameOnly` _returnvalue)
  (set `PlayerController.bShowMouseCursor` false _returnvalue))

(fn `UserConstructionScript`)